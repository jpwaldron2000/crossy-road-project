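; Lane spawner actor that builds a chain of randomly chosen lane types, starting at the player pawn on BeginPlay.
; SpawnLane re-rolls at each branch, so odds are uneven and a call can spawn nothing; BP_Lane1 and BP_Lane12 alternate.
; Each lane gets a spawner reference, and LastLane selects whose SpawnPoint places the next.
; The initial loop's switch is fixed at 0, so it spawns at the pawn until a BP_Lane exists.
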(event EventBeginPlay
  (CallFunction|SpawnInitialLanes))

(fn ConstructionScript)

(fn SpawnLane
  (params (SpawnLocation :type Vector))
  (bind _returnvalue (Math|Random|RandomIntegerinRange 0 3))
  (if (== _returnvalue 0)
    (bind _returnvalue_2 (Game|SpawnActorfromClass "/Game/Blueprints/BP_Lane.BP_Lane_C" (Math|Transform|MakeTransform SpawnLocation "0, 0, 0" "4.000000,2.000000,2.000000") "Undefined" 0 0))
    (bind _output_get (Variables|Default|SetNewestLane _returnvalue_2))
    (Variables|/Game/Blueprints/BP_Lane.BP_Lane_C|SetLaneSpawner _output_get self)
    (Variables|Default|SetlastLane 0)
    (elif (== _returnvalue 1)
      (if (Variables|Default|Getgrass%20alternator)
        (bind _returnvalue_3 (Game|SpawnActorfromClass "/Game/Blueprints/BP_Lane1.BP_Lane1_C" (Math|Transform|MakeTransform SpawnLocation "0, 0, 0" "4.000000,2.000000,2.000000") "Undefined" 0 0))
        (bind _output_get_2 (Variables|Default|SetNewestLane1 _returnvalue_3))
        (Variables|/Game/Blueprints/BP_Lane1.BP_Lane1_C|SetLaneSpawner1 _output_get_2 self)
        (Variables|Default|SetlastLane 1)
        (Variables|Default|Setgrass%20alternator false)
        (else
          (bind _returnvalue_4 (Game|SpawnActorfromClass "/Game/Blueprints/BP_Lane12.BP_Lane12_C" (Math|Transform|MakeTransform SpawnLocation "0, 0, 0" "4.000000,2.000000,2.000000") "Undefined" 0 0))
          (bind _output_get_3 (Variables|Default|SetNewestLane12 _returnvalue_4))
          (Variables|/Game/Blueprints/BP_Lane12.BP_Lane12_C|SetLaneSpawner1 _output_get_3 self)
          (Variables|Default|SetlastLane 4)
          (Variables|Default|Setgrass%20alternator true)))
      (elif (== _returnvalue 2)
        (bind _returnvalue_5 (Game|SpawnActorfromClass "/Game/Blueprints/BP_Lane2.BP_Lane2_C" (Math|Transform|MakeTransform SpawnLocation "0, 0, 0" "4.000000,2.000000,2.000000") "Undefined" 0 0))
        (bind _output_get_4 (Variables|Default|SetNewestLane2 _returnvalue_5))
        (Variables|/Game/Blueprints/BP_Lane2.BP_Lane2_C|SetLaneSpawner2 _output_get_4 self)
        (Variables|Default|SetlastLane 2)
        (elif (== _returnvalue 3)
          (bind _returnvalue_6 (Game|SpawnActorfromClass "/Game/Blueprints/BP_Lane3.BP_Lane3_C" (Math|Transform|MakeTransform SpawnLocation "0, 0, 0" "4.000000,2.000000,2.000000") "Undefined" 0 0))
          (bind _output_get_5 (Variables|Default|SetNewestLane3 _returnvalue_6))
          (Variables|/Game/Blueprints/BP_Lane3.BP_Lane3_C|SetLaneSpawner3 _output_get_5 self)
          (Variables|Default|SetlastLane 3))))))

(fn SpawnLaneatSpawnPoint
  (bind _newestlane (Variables|Default|GetNewestLane))
  (bind _newestlane1 (Variables|Default|GetNewestLane1))
  (bind _newestlane2 (Variables|Default|GetNewestLane2))
  (bind _newestlane12 (Variables|Default|GetNewestLane12))
  (bind _newestlane3 (Variables|Default|GetNewestLane3))
  (bind _spawnpoint (Variables|/Game/Blueprints/BP_Lane12.BP_Lane12_C|GetSpawnPoint _newestlane12))
  (bind _spawnpoint_2 (Variables|/Game/Blueprints/BP_Lane.BP_Lane_C|GetSpawnPoint _newestlane))
  (bind _spawnpoint_3 (Variables|/Game/Blueprints/BP_Lane1.BP_Lane1_C|GetSpawnPoint _newestlane1))
  (bind _spawnpoint_4 (Variables|/Game/Blueprints/BP_Lane2.BP_Lane2_C|GetSpawnPoint _newestlane2))
  (bind _spawnpoint_5 (Variables|/Game/Blueprints/BP_Lane3.BP_Lane3_C|GetSpawnPoint _newestlane3))
  (bind _returnvalue (Transformation|GetWorldLocation _spawnpoint_2))
  (bind _returnvalue_2 (Transformation|GetWorldLocation _spawnpoint))
  (bind _returnvalue_3 (Transformation|GetWorldLocation _spawnpoint_4))
  (bind _returnvalue_4 (Transformation|GetWorldLocation _spawnpoint_3))
  (bind _returnvalue_5 (Transformation|GetWorldLocation _spawnpoint_5))
  (switch int (Variables|Default|GetlastLane)
    (:0
      (CallFunction|SpawnLane (Math|Vector|MakeVector (.x _returnvalue) (.y _returnvalue) 1e+01)))
    (:1
      (CallFunction|SpawnLane (Math|Vector|MakeVector (.x _returnvalue_4) (.y _returnvalue_4) 1e+01)))
    (:2
      (CallFunction|SpawnLane (Math|Vector|MakeVector (.x _returnvalue_3) (.y _returnvalue_3) 1e+01)))
    (:3
      (CallFunction|SpawnLane (Math|Vector|MakeVector (.x _returnvalue_5) (.y _returnvalue_5) 1e+01)))
    (:4
      (CallFunction|SpawnLane (Math|Vector|MakeVector (.x _returnvalue_2) (.y _returnvalue_2) 1e+01)))))

(fn SpawnInitialLanes
  (bind _returnvalue (Game|Player|GetPlayerPawn 0))
  (bind _returnvalue_2 (Game|Player|GetPlayerPawn 0))
  (bind _returnvalue_3 (Game|Player|GetPlayerPawn 0))
  (bind _returnvalue_4 (Game|Player|GetPlayerPawn 0))
  (bind _returnvalue_5 (Game|Player|GetPlayerPawn 0))
  (bind _returnvalue_6 (Transformation|GetActorLocation _returnvalue_2))
  (bind _returnvalue_7 (Transformation|GetActorLocation _returnvalue_3))
  (bind _returnvalue_8 (Transformation|GetActorLocation _returnvalue))
  (bind _returnvalue_9 (Transformation|GetActorLocation _returnvalue_4))
  (bind _returnvalue_10 (Transformation|GetActorLocation _returnvalue_5))
  (for _index (range 0 10)
    (switch int 0
      (:0
        (Utilities|IsValid (Variables|Default|GetNewestLane)
          (:Is%20Valid
            (CallFunction|SpawnLaneatSpawnPoint))
          (:Is%20Not%20Valid
            (CallFunction|SpawnLane (Math|Vector|MakeVector (.x _returnvalue_6) (.y _returnvalue_6) 1e+01)))))
      (:1
        (Utilities|IsValid (Variables|Default|GetNewestLane1)
          (:Is%20Valid
            (CallFunction|SpawnLaneatSpawnPoint))
          (:Is%20Not%20Valid
            (CallFunction|SpawnLane (Math|Vector|MakeVector (.x _returnvalue_7) (.y _returnvalue_7) 1e+01)))))
      (:2
        (Utilities|IsValid (Variables|Default|GetNewestLane2)
          (:Is%20Valid
            (CallFunction|SpawnLaneatSpawnPoint))
          (:Is%20Not%20Valid
            (CallFunction|SpawnLane (Math|Vector|MakeVector (.x _returnvalue_10) (.y _returnvalue_10) 1e+01)))))
      (:3
        (Utilities|IsValid (Variables|Default|GetNewestLane3)
          (:Is%20Valid
            (CallFunction|SpawnLaneatSpawnPoint))
          (:Is%20Not%20Valid
            (CallFunction|SpawnLane (Math|Vector|MakeVector (.x _returnvalue_8) (.y _returnvalue_8) 1e+01)))))
      (:4
        (Utilities|IsValid (Variables|Default|GetNewestLane12)
          (:Is%20Valid
            (CallFunction|SpawnLaneatSpawnPoint))
          (:Is%20Not%20Valid
            (CallFunction|SpawnLane (Math|Vector|MakeVector (.x _returnvalue_9) (.y _returnvalue_9) 1e+01))))))))