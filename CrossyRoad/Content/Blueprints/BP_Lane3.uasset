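; BP_Lane3 is a railway lane that spawns a single BP_Train from a randomly chosen end after a random timer set at BeginPlay.
; While the spawn sequence runs, Tick uses delays to toggle two warning lights and play a railroad sound.
; End colliders destroy arriving trains, and a player overlapping TriggerZone tells LaneSpawner3 to spawn another lane.
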(event OnComponentBeginOverlap(TriggerZone)
  (params (OverlappedComponent :type Primitive%20Component%20Object%20Reference) (OtherActor :type Actor%20Object%20Reference) (OtherComp :type Primitive%20Component%20Object%20Reference) (OtherBodyIndex :type Integer) (bFromSweep :type Boolean) (SweepResult :type Hit%20Result%20Structure%20%28by%20ref%29))
  (Utilities|Casting|CastToBP_Player OtherActor)
  (Default|SpawnLaneatSpawnPoint (Variables|Default|GetLaneSpawner3)))

(event OnComponentBeginOverlap(CarCollider2)
  (params (OverlappedComponent :type Primitive%20Component%20Object%20Reference) (OtherActor :type Actor%20Object%20Reference) (OtherComp :type Primitive%20Component%20Object%20Reference) (OtherBodyIndex :type Integer) (bFromSweep :type Boolean) (SweepResult :type Hit%20Result%20Structure%20%28by%20ref%29))
  (bind _asbp_train (Utilities|Casting|CastToBP_Train OtherActor))
  (Actor|DestroyActor _asbp_train))

(event OnComponentBeginOverlap(CarCollider1)
  (params (OverlappedComponent :type Primitive%20Component%20Object%20Reference) (OtherActor :type Actor%20Object%20Reference) (OtherComp :type Primitive%20Component%20Object%20Reference) (OtherBodyIndex :type Integer) (bFromSweep :type Boolean) (SweepResult :type Hit%20Result%20Structure%20%28by%20ref%29))
  (bind _asbp_train (Utilities|Casting|CastToBP_Train OtherActor))
  (Actor|DestroyActor _asbp_train))

(event Custom|trainSpawn
  (Variables|Default|SettrainSpawning true)
  (Utilities|FlowControl|Delay 2.0)
  (if (Variables|Default|GetstartingLocation)
    (Game|SpawnActorfromClass "/Game/Blueprints/BP_Train.BP_Train_C" (Math|Transform|MakeTransform (Variables|Default|GetstartLocation) "0, 0, 0" "1.000000,1.000000,1.000000") "Undefined" 0 0)
    (Utilities|FlowControl|Delay 2.0)
    (Variables|Default|SettrainSpawning false)
    (else
      (Game|SpawnActorfromClass "/Game/Blueprints/BP_Train.BP_Train_C" (Math|Transform|MakeTransform (Variables|Default|GetendLocation) "0,180.000000, 0" "1.000000,1.000000,1.000000") "Undefined" 0 0)
      (Utilities|FlowControl|Delay 2.0)
      (Variables|Default|SettrainSpawning false))))

(event EventBeginPlay
  (Variables|Default|SetendLocation (Transformation|GetWorldLocation (Variables|Default|Getend)))
  (Variables|Default|SetstartLocation (Transformation|GetWorldLocation (Variables|Default|Getstart)))
  (Variables|Default|SetstartingLocation (Math|Random|RandomBool))
  (Utilities|Time|SetTimerbyEvent (delegate Custom|trainSpawn) (Math|Random|RandomFloatinRange 5.0 1e+01)))

(event EventTick
  (params (DeltaSeconds :type Float%20%28single-precision%29))
  (if (Variables|Default|GettrainSpawning)
    (Utilities|FlowControl|Delay 1.0)
    (Rendering|ToggleVisibility (Variables|Default|GetleftLight) false)
    (Utilities|FlowControl|Delay 1.0)
    (Rendering|ToggleVisibility (Variables|Default|GetrightLight) false)
    (Audio|PlaySoundatLocation "/Game/Sounds/railroad.railroad" (Transformation|GetActorLocation) "0, 0, 0" 1.0 1.0 0.0 0 0 0 0)))

(fn ConstructionScript)