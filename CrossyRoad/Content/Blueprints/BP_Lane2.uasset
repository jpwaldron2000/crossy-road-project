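; BP_Lane2 is a water lane where logs spawn and the player dies on falling in.
; At BeginPlay it randomly picks the Start or End side, then spawns BP_Log there on a looping timer, with the interval randomized once and End-side logs rotated 180 degrees.
; Two colliders destroy logs that reach them.
; Player overlaps drive the rest: TriggerZone has LaneSpawner2 spawn another lane, while Deathbox calls Waterdead and plays a splash.
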(event OnComponentBeginOverlap(TriggerZone)
  (params (OverlappedComponent :type Primitive%20Component%20Object%20Reference) (OtherActor :type Actor%20Object%20Reference) (OtherComp :type Primitive%20Component%20Object%20Reference) (OtherBodyIndex :type Integer) (bFromSweep :type Boolean) (SweepResult :type Hit%20Result%20Structure%20%28by%20ref%29))
  (Utilities|Casting|CastToBP_Player OtherActor)
  (Default|SpawnLaneatSpawnPoint (Variables|Default|GetLaneSpawner2)))

(event OnComponentBeginOverlap(LogCollider1)
  (params (OverlappedComponent :type Primitive%20Component%20Object%20Reference) (OtherActor :type Actor%20Object%20Reference) (OtherComp :type Primitive%20Component%20Object%20Reference) (OtherBodyIndex :type Integer) (bFromSweep :type Boolean) (SweepResult :type Hit%20Result%20Structure%20%28by%20ref%29))
  (bind _asbp_log (Utilities|Casting|CastToBP_Log OtherActor))
  (Actor|DestroyActor _asbp_log))

(event OnComponentBeginOverlap(LogCollider2)
  (params (OverlappedComponent :type Primitive%20Component%20Object%20Reference) (OtherActor :type Actor%20Object%20Reference) (OtherComp :type Primitive%20Component%20Object%20Reference) (OtherBodyIndex :type Integer) (bFromSweep :type Boolean) (SweepResult :type Hit%20Result%20Structure%20%28by%20ref%29))
  (bind _asbp_log (Utilities|Casting|CastToBP_Log OtherActor))
  (Actor|DestroyActor _asbp_log))

(event OnComponentBeginOverlap(deathbox)
  (params (OverlappedComponent :type Primitive%20Component%20Object%20Reference) (OtherActor :type Actor%20Object%20Reference) (OtherComp :type Primitive%20Component%20Object%20Reference) (OtherBodyIndex :type Integer) (bFromSweep :type Boolean) (SweepResult :type Hit%20Result%20Structure%20%28by%20ref%29))
  (bind _asbp_player (Utilities|Casting|CastToBP_Player OtherActor))
  (Default|Waterdead _asbp_player)
  (Audio|PlaySoundatLocation "/Game/Sounds/splash.splash" (Transformation|GetWorldLocation (Variables|/Game/Blueprints/BP_Player.BP_Player_C|Getplayer _asbp_player)) "0, 0, 0" 1.0 1.0 0.0 0 0 0 0))

(event Custom|spawn%20logs
  (if (Variables|Default|Getstarting%20Location)
    (Game|SpawnActorfromClass "/Game/Blueprints/BP_Log.BP_Log_C" (Math|Transform|MakeTransform (Variables|Default|Getstart_Location) "0, 0, 0" "1.000000,1.000000,1.000000") "Undefined" 0 0)
    (else
      (Game|SpawnActorfromClass "/Game/Blueprints/BP_Log.BP_Log_C" (Math|Transform|MakeTransform (Variables|Default|GetendLocation) "0,180.000000, 0" "1.000000,1.000000,1.000000") "Undefined" 0 0))))

(event EventBeginPlay
  (Variables|Default|SetendLocation (Transformation|GetWorldLocation (Variables|Default|Getend)))
  (Variables|Default|Setstart_Location (Transformation|GetWorldLocation (Variables|Default|Getstart)))
  (Variables|Default|Setstarting%20Location (Math|Random|RandomBool))
  (Utilities|Time|SetTimerbyEvent (delegate Custom|spawn%20logs) (Math|Random|RandomFloatinRange 3.0 5.0) true))

(fn ConstructionScript)