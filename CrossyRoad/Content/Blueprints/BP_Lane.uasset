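; BP_Lane is a road lane that spawns traffic and a coin, and extends the level through LaneSpawner when the player enters its trigger zone.
; BeginPlay places a coin at a random X offset, picks a random traffic side and starts a looping spawn timer with a randomized interval.
; The Start side spawns ambulances or trucks at random, while the End side spawns only rotated ambulances.
; Two end colliders destroy overlapping actors.
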(event OnComponentBeginOverlap(TriggerZone)
  (params (OverlappedComponent :type Primitive%20Component%20Object%20Reference) (OtherActor :type Actor%20Object%20Reference) (OtherComp :type Primitive%20Component%20Object%20Reference) (OtherBodyIndex :type Integer) (bFromSweep :type Boolean) (SweepResult :type Hit%20Result%20Structure%20%28by%20ref%29))
  (Utilities|Casting|CastToBP_Player OtherActor)
  (Default|SpawnLaneatSpawnPoint (Variables|Default|GetLaneSpawner)))

(event OnComponentBeginOverlap(CarCollider1)
  (params (OverlappedComponent :type Primitive%20Component%20Object%20Reference) (OtherActor :type Actor%20Object%20Reference) (OtherComp :type Primitive%20Component%20Object%20Reference) (OtherBodyIndex :type Integer) (bFromSweep :type Boolean) (SweepResult :type Hit%20Result%20Structure%20%28by%20ref%29))
  (Actor|DestroyActor OtherActor))

(event OnComponentBeginOverlap(CarCollider2)
  (params (OverlappedComponent :type Primitive%20Component%20Object%20Reference) (OtherActor :type Actor%20Object%20Reference) (OtherComp :type Primitive%20Component%20Object%20Reference) (OtherBodyIndex :type Integer) (bFromSweep :type Boolean) (SweepResult :type Hit%20Result%20Structure%20%28by%20ref%29))
  (Actor|DestroyActor OtherActor))

(event Custom|spawn%20vehicles
  (bind _startlocation (Variables|Default|GetstartLocation))
  (bind _endlocation (Variables|Default|GetendLocation))
  (if (Variables|Default|GetstartingLocation)
    (if (Math|Random|RandomBool)
      (Game|SpawnActorfromClass "/Game/Blueprints/BP_Ambulance.BP_Ambulance_C" (Math|Transform|MakeTransform _startlocation "0, 0, 0" "1.000000,1.000000,1.000000") "Undefined" 0 0)
      (else
        (Game|SpawnActorfromClass "/Game/Blueprints/BP_Truck.BP_Truck_C" (Math|Transform|MakeTransform _startlocation "0, 0, 0" "1.000000,1.000000,1.000000") "Undefined" 0 0)))
    (elif true
      (Game|SpawnActorfromClass "/Game/Blueprints/BP_Ambulance.BP_Ambulance_C" (Math|Transform|MakeTransform _endlocation "0,180.000000, 0" "1.000000,1.000000,1.000000") "Undefined" 0 0)
      (else
        (Game|SpawnActorfromClass "/Game/Blueprints/BP_Truck.BP_Truck_C" (Math|Transform|MakeTransform _endlocation "0,180.000000, 0" "1.000000,1.000000,1.000000") "Undefined" 0 0)))))

(event EventBeginPlay
  (Variables|Default|SetstartLocation (Transformation|GetWorldLocation (Variables|Default|Getstart)))
  (Variables|Default|SetendLocation (Transformation|GetWorldLocation (Variables|Default|Getend)))
  (Game|SpawnActorfromClass "/Game/Blueprints/BP_Coin.BP_Coin_C" (Math|Transform|MakeTransform (Math|Vector|MakeVector (+ (.x (Variables|Default|GetstartLocation)) (Math|Random|RandomFloatinRange 0.0 2e+03)) (.y (Variables|Default|GetstartLocation)) 4e+01) "0, 0, 0" "1.000000,1.000000,1.000000") "Undefined" 0 0)
  (Variables|Default|SetstartingLocation (Math|Random|RandomBool))
  (Utilities|Time|SetTimerbyEvent (delegate Custom|spawn%20vehicles) (Math|Random|RandomFloatinRange 3.0 5.0) true))

(fn ConstructionScript)