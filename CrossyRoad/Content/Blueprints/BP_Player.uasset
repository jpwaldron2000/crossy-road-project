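; Player character for a Crossy Road-style chicken hopper with step and coin high scores.
; Axis input launches cooldown-gated hops and turns the mesh; forward and right hops increment the step counter on the BP_UI widget.
; High scores load at BeginPlay and save to SaveGameHS only on the random cluck branch of those hops.
; Vehicle hits, water deaths and CameraBox overlaps stop the moving camera and show GameOver.
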(event OnComponentBeginOverlap(camerabox)
  (params (OverlappedComponent :type Primitive%20Component%20Object%20Reference) (OtherActor :type Actor%20Object%20Reference) (OtherComp :type Primitive%20Component%20Object%20Reference) (OtherBodyIndex :type Integer) (bFromSweep :type Boolean) (SweepResult :type Hit%20Result%20Structure%20%28by%20ref%29))
  (if (Collision|IsOverlappingActor (Variables|Default|Getcamera%20box) OtherActor :!class /Script/Engine.PrimitiveComponent)
    (Audio|PlaySoundatLocation "/Game/Sounds/eagle.eagle" (Transformation|GetWorldLocation (Variables|Default|Getplayer)) "0, 0, 0" 1.0 1.0 0.0 0 0 0 0)
    (Components|Movement|StopMovementImmediately (Variables|Default|GetCameraMove))
    (bind _returnvalue (UserInterface|CreateWidget "/Game/Blueprints/GameOver.GameOver_C"))
    (UserInterface|Viewport|AddtoViewport _returnvalue 0)
    (Variables|/Script/Engine.PlayerController|SetbShowMouseCursor (Game|GetPlayerController 0) true)
    (Variables|/Script/Engine.CharacterMovementComponent|SetMaxWalkSpeed (Variables|Character|GetCharacterMovement) 0.0)))

(event Custom|MovementCoolDown
  ;[0.2776 1 0.9303] Move Cool Down
  (Utilities|FlowControl|DoOnce false :!label _label
    (:Completed
      (Variables|Default|SetCanMove false)
      (Utilities|FlowControl|Delay 0.5)
      (Variables|Default|SetCanMove true)
      (goto _label Reset))))

(event Custom|HitbyVehicle
  ;[1 0.2031 0.2031] Player Killed
  (Transformation|SetWorldScale3D (Variables|Default|Getplayer) "1.000000,1.000000,0.100000")
  (Components|Movement|StopMovementImmediately (Variables|Default|GetCameraMove))
  (bind _returnvalue (UserInterface|CreateWidget "/Game/Blueprints/GameOver.GameOver_C"))
  (UserInterface|Viewport|AddtoViewport _returnvalue 0)
  (Variables|/Script/Engine.PlayerController|SetbShowMouseCursor (Game|GetPlayerController 0) true)
  (Variables|/Script/Engine.CharacterMovementComponent|SetMaxWalkSpeed (Variables|Character|GetCharacterMovement) 0.0))

(event Custom|waterdead
  ;[1 0.2031 0.2031] Player Killed
  (Components|Activation|Activate (Variables|Default|Getparticles) false)
  (Components|Movement|StopMovementImmediately (Variables|Default|GetCameraMove))
  (bind _returnvalue (UserInterface|CreateWidget "/Game/Blueprints/GameOver.GameOver_C"))
  (UserInterface|Viewport|AddtoViewport _returnvalue 0)
  (Variables|/Script/Engine.PlayerController|SetbShowMouseCursor (Game|GetPlayerController 0) true)
  (Variables|/Script/Engine.CharacterMovementComponent|SetMaxWalkSpeed (Variables|Character|GetCharacterMovement) 0.0))

(event EventBeginPlay
  (bind _slot_name (Variables|Default|GetSlot%20Name))
  ;[0.1996 1 0.3151] Begin Play
  (Components|Movement|SetUpdatedComponent (Variables|Default|GetCameraMove) (Variables|Default|GetCameraBoom))
  (bind _returnvalue (SaveGame|DoesSaveGameExist _slot_name))
  (if _returnvalue
    (bind _returnvalue_2 (SaveGame|LoadGamefromSlot _slot_name))
    (bind _output_get (Variables|Default|SetSaver%20Subclass _returnvalue_2))
    (bind _assave_game_hs (Utilities|Casting|CastToSaveGameHS _output_get))
    (Variables|Default|SetCoinHighScore (Variables|/Game/Blueprints/SaveGameHS.SaveGameHS_C|GetCoinHS _assave_game_hs))
    (Variables|Default|SetStepHighScore (Variables|/Game/Blueprints/SaveGameHS.SaveGameHS_C|GetStepHS _assave_game_hs)))
  (bind _returnvalue_3 (Game|ConstructObjectfromClass "/Game/Blueprints/BP_UI.BP_UI_C"))
  (UserInterface|Viewport|AddtoViewport _returnvalue_3 0)
  (Variables|/Game/Blueprints/BP_UI.BP_UI_C|SetplayerRef _returnvalue_3 self)
  (bind _output_get_2 (Variables|Default|SetBP_UI _returnvalue_3))
  (Default|UpdateStepCounter _output_get_2))

(event Input|AxisEvents|InputAxisMoveForward
  (params (AxisValue :type Float%20%28single-precision%29))
  ;[1 0.8152 0.2044] Character Movement and score stuff
  (if (and (> (Math|Float|Absolute(Float) AxisValue) 0.3) (Variables|Default|GetCanMove))
    (CallFunction|MovementCoolDown)
    (Character|LaunchCharacter (Math|Vector|MakeVector 0.0 (* AxisValue 2.4e+02) 2e+02) true true)
    (if (> AxisValue 0.3)
      (Transformation|SetWorldRotation (Variables|Default|Getplayer) "0,0.000000, 0" false false)
      (Math|Integer|IncrementInt (Variables|Default|GetStepCounter)
        (:%20%20
          (Default|UpdateStepCounter (Variables|Default|GetBP_UI))
          (switch int (Math|Random|RandomInteger 2)
            (:0
              (Audio|PlaySoundatLocation "/Game/Sounds/cluck.cluck" (Transformation|GetActorLocation) "0, 0, 0" 1.0 1.0 0.0 0 0 0 0)
              (if (> (Variables|Default|GetStepCounter) (Variables|Default|GetStepHighScore))
                (Variables|Default|SetStepHighScore (Variables|Default|GetStepCounter)))
              (if (> (Variables|Default|GetCoinCounter1) (Variables|Default|GetCoinHighScore))
                (Variables|Default|SetCoinHighScore (Variables|Default|GetCoinCounter1)))
              (bind _returnvalue (SaveGame|DoesSaveGameExist (Variables|Default|GetSlot%20Name)))
              (if _returnvalue
                (bind _returnvalue_2 (SaveGame|LoadGamefromSlot (Variables|Default|GetSlot%20Name)))
                (bind _output_get (Variables|Default|SetSaver%20Subclass _returnvalue_2))
                (bind _assave_game_hs (Utilities|Casting|CastToSaveGameHS _output_get))
                (Variables|/Game/Blueprints/SaveGameHS.SaveGameHS_C|SetStepHS _assave_game_hs (Variables|Default|GetStepHighScore))
                (Variables|/Game/Blueprints/SaveGameHS.SaveGameHS_C|SetCoinHS _assave_game_hs (Variables|Default|GetCoinHighScore))
                (SaveGame|SaveGametoSlot (Variables|Default|GetSaver%20Subclass) (Variables|Default|GetSlot%20Name))
                (else
                  (bind _returnvalue_3 (SaveGame|CreateSaveGameObject "/Game/Blueprints/SaveGameHS.SaveGameHS_C"))
                  (bind _output_get_2 (Variables|Default|SetSaver%20Subclass _returnvalue_3))
                  (bind _assave_game_hs_2 (Utilities|Casting|CastToSaveGameHS _output_get_2))
                  (Variables|/Game/Blueprints/SaveGameHS.SaveGameHS_C|SetStepHS _assave_game_hs_2 (Variables|Default|GetStepHighScore))
                  (Variables|/Game/Blueprints/SaveGameHS.SaveGameHS_C|SetCoinHS _assave_game_hs_2 (Variables|Default|GetCoinHighScore))
                  (SaveGame|SaveGametoSlot (Variables|Default|GetSaver%20Subclass) (Variables|Default|GetSlot%20Name))))))))
      (else
        (Transformation|SetWorldRotation (Variables|Default|Getplayer) "0,180.000000, 0" false false)))))

(event Input|AxisEvents|InputAxisMoveRight
  (params (AxisValue :type Float%20%28single-precision%29))
  ;[1 0.8152 0.2044] Character Movement and score stuff
  (if (and (> (Math|Float|Absolute(Float) AxisValue) 0.3) (Variables|Default|GetCanMove))
    (CallFunction|MovementCoolDown)
    (Character|LaunchCharacter (Math|Vector|MakeVector (* AxisValue 2.4e+02) 0.0 2e+02) true true)
    (if (> AxisValue 0.3)
      (Transformation|SetWorldRotation (Variables|Default|Getplayer) "0,270.000000, 0" false false)
      (Math|Integer|IncrementInt (Variables|Default|GetStepCounter)
        (:%20%20
          (Default|UpdateStepCounter (Variables|Default|GetBP_UI))
          (switch int (Math|Random|RandomInteger 2)
            (:0
              (Audio|PlaySoundatLocation "/Game/Sounds/cluck.cluck" (Transformation|GetActorLocation) "0, 0, 0" 1.0 1.0 0.0 0 0 0 0)
              (if (> (Variables|Default|GetStepCounter) (Variables|Default|GetStepHighScore))
                (Variables|Default|SetStepHighScore (Variables|Default|GetStepCounter)))
              (if (> (Variables|Default|GetCoinCounter1) (Variables|Default|GetCoinHighScore))
                (Variables|Default|SetCoinHighScore (Variables|Default|GetCoinCounter1)))
              (bind _returnvalue (SaveGame|DoesSaveGameExist (Variables|Default|GetSlot%20Name)))
              (if _returnvalue
                (bind _returnvalue_2 (SaveGame|LoadGamefromSlot (Variables|Default|GetSlot%20Name)))
                (bind _output_get (Variables|Default|SetSaver%20Subclass _returnvalue_2))
                (bind _assave_game_hs (Utilities|Casting|CastToSaveGameHS _output_get))
                (Variables|/Game/Blueprints/SaveGameHS.SaveGameHS_C|SetStepHS _assave_game_hs (Variables|Default|GetStepHighScore))
                (Variables|/Game/Blueprints/SaveGameHS.SaveGameHS_C|SetCoinHS _assave_game_hs (Variables|Default|GetCoinHighScore))
                (SaveGame|SaveGametoSlot (Variables|Default|GetSaver%20Subclass) (Variables|Default|GetSlot%20Name))
                (else
                  (bind _returnvalue_3 (SaveGame|CreateSaveGameObject "/Game/Blueprints/SaveGameHS.SaveGameHS_C"))
                  (bind _output_get_2 (Variables|Default|SetSaver%20Subclass _returnvalue_3))
                  (bind _assave_game_hs_2 (Utilities|Casting|CastToSaveGameHS _output_get_2))
                  (Variables|/Game/Blueprints/SaveGameHS.SaveGameHS_C|SetStepHS _assave_game_hs_2 (Variables|Default|GetStepHighScore))
                  (Variables|/Game/Blueprints/SaveGameHS.SaveGameHS_C|SetCoinHS _assave_game_hs_2 (Variables|Default|GetCoinHighScore))
                  (SaveGame|SaveGametoSlot (Variables|Default|GetSaver%20Subclass) (Variables|Default|GetSlot%20Name))))))))
      (else
        (Transformation|SetWorldRotation (Variables|Default|Getplayer) "0,90.000000, 0" false false)))))

(fn ConstructionScript)

(fn NewFunction0)