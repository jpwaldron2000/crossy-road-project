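; BP_Police is a police Blueprint with rotating red and blue lights.
; Each tick it adds SpinSpeed to the world yaw of both RedLight and BlueLight while keeping their roll and pitch.
; The spin is applied per frame without delta time scaling, so its speed depends on frame rate.
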(event EventTick
  (params (DeltaSeconds :type Float%20%28single-precision%29))
  (bind _redlight (Variables|Default|GetredLight))
  (bind _bluelight (Variables|Default|GetblueLight))
  (bind _returnvalue (Transformation|GetSocketRotation _redlight "None"))
  (bind _returnvalue_2 (Transformation|GetSocketRotation _bluelight "None"))
  (Transformation|SetWorldRotation (Variables|Default|GetredLight) (Math|Rotator|MakeRotator (.roll _returnvalue) (.pitch _returnvalue) (+ (.yaw _returnvalue) (Variables|Default|Getspin%20speed))) false false)
  (Transformation|SetWorldRotation (Variables|Default|GetblueLight) (Math|Rotator|MakeRotator (.roll _returnvalue_2) (.pitch _returnvalue_2) (+ (.yaw _returnvalue_2) (Variables|Default|Getspin%20speed))) false false))

(fn ConstructionScript)