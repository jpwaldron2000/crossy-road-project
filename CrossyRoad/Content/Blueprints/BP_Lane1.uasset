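; BP_Lane1 is a lane segment that populates itself with obstacles and a coin, then extends the level as the player advances.
; On BeginPlay, a loop sized by the Start-to-End distance steps along X, randomly spawning BP_TreeandRock, with a DoOnce allowing at most one BP_Coin.
; A BP_Player overlap on TriggerZone calls LaneSpawner1 to spawn another lane.
; A BP_Ambulance overlap on either car collider destroys this lane actor.
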(event OnComponentBeginOverlap(TriggerZone)
  (params (OverlappedComponent :type Primitive%20Component%20Object%20Reference) (OtherActor :type Actor%20Object%20Reference) (OtherComp :type Primitive%20Component%20Object%20Reference) (OtherBodyIndex :type Integer) (bFromSweep :type Boolean) (SweepResult :type Hit%20Result%20Structure%20%28by%20ref%29))
  (Utilities|Casting|CastToBP_Player OtherActor)
  (Default|SpawnLaneatSpawnPoint (Variables|Default|GetLaneSpawner1)))

(event OnComponentBeginOverlap(CarCollider2)
  (params (OverlappedComponent :type Primitive%20Component%20Object%20Reference) (OtherActor :type Actor%20Object%20Reference) (OtherComp :type Primitive%20Component%20Object%20Reference) (OtherBodyIndex :type Integer) (bFromSweep :type Boolean) (SweepResult :type Hit%20Result%20Structure%20%28by%20ref%29))
  (Utilities|Casting|CastToBP_Ambulance OtherActor)
  (Actor|DestroyActor))

(event OnComponentBeginOverlap(CarCollider1)
  (params (OverlappedComponent :type Primitive%20Component%20Object%20Reference) (OtherActor :type Actor%20Object%20Reference) (OtherComp :type Primitive%20Component%20Object%20Reference) (OtherBodyIndex :type Integer) (bFromSweep :type Boolean) (SweepResult :type Hit%20Result%20Structure%20%28by%20ref%29))
  (Utilities|Casting|CastToBP_Ambulance OtherActor)
  (Actor|DestroyActor))

(event EventBeginPlay
  (Variables|Default|SetstartLocation (Transformation|GetWorldLocation (Variables|Default|Getstart)))
  (Variables|Default|SetendLocation (Transformation|GetWorldLocation (Variables|Default|Getend)))
  (for _index (range 0 (Math|Float|Truncate (/ (Math|Vector|Distance(Vector) (Variables|Default|GetstartLocation) (Variables|Default|GetendLocation)) 1e+01)))
    (if (> (Math|Random|RandomIntegerinRange 0 100) 80)
      (Game|SpawnActorfromClass "/Game/Blueprints/BP_TreeandRock.BP_TreeandRock_C" (Math|Transform|MakeTransform (Math|Vector|MakeVector (+ (* _index 50) (.x (Variables|Default|GetstartLocation))) (.y (Variables|Default|GetstartLocation)) (.z (Variables|Default|GetstartLocation))) "0, 0, 0" "1.000000,1.000000,1.000000") "Undefined" 0 0)
      (elif (Math|Random|RandomBool)
        (Utilities|FlowControl|DoOnce false
          (:Completed
            (Game|SpawnActorfromClass "/Game/Blueprints/BP_Coin.BP_Coin_C" (Math|Transform|MakeTransform (Math|Vector|MakeVector (+ (* _index 50) (.x (Variables|Default|GetstartLocation))) (.y (Variables|Default|GetstartLocation)) 4e+01) "0, 0, 0" "1.000000,1.000000,1.000000") "Undefined" 0 0)))))))

(fn ConstructionScript)