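; BP_Light is a railroad warning light actor that reacts to an approaching train.
; Each Tick it checks TrainSpawning on its TrainRef and, when true, toggles the right light, then the left light, with one-second delays between them.
; After the left toggle it plays the Railroad sound at the actor's location, so the blink and sound repeat while spawning stays true.
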(event EventTick
  (params (DeltaSeconds :type Float%20%28single-precision%29))
  (if (Variables|/Game/Blueprints/BP_Lane3.BP_Lane3_C|GettrainSpawning (Variables|Default|GetTrain%20Ref))
    (Utilities|FlowControl|Delay 1.0)
    (Rendering|ToggleVisibility (Variables|Default|Getright_light1) false)
    (Utilities|FlowControl|Delay 1.0)
    (Rendering|ToggleVisibility (Variables|Default|Getleft_light) false)
    (Audio|PlaySoundatLocation "/Game/Sounds/railroad.railroad" (Transformation|GetActorLocation) "0, 0, 0" 1.0 1.0 0.0 0 0 0 0)))

(fn ConstructionScript)